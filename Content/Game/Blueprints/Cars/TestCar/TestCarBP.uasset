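; Drivable rear-wheel-drive test car with a component-based custom drivetrain simulation, three switchable cameras and on-screen telemetry.
; Each tick, torque flows from engine through clutch, gearbox and differential to rear wheels, while wheel velocities feed back to set clutch and engine load.
; Input drives smoothed steering, throttle and biased brakes with rear handbrake, plus shifting and a held torque boost.
; Construction-spawned wheel meshes follow suspension length and wheel spin.
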(event EventBeginPlay
  (Default|Initialize (Variables|Default|GetWheel_FR) (Variables|Default|GetBody)))

(event EventTick
  (params (DeltaSeconds :type Float%20%28single-precision%29))
  (bind _clutch (Variables|Default|GetClutch))
  (bind _gearbox (Variables|Default|GetGearBox))
  (bind _body (Variables|Default|GetBody))
  (bind _breaktorque (Variables|Break|GetBreakTorque))
  (bind _boost (Variables|Default|GetBoost))
  (bind _engine (Variables|Default|GetEngine))
  (bind _output (Utilities|Array|Get(acopy) _breaktorque))
  (bind _output_2 (Utilities|Array|Get(acopy) _breaktorque 1))
  (bind _output_get (Variables|Default|SetDelta%20Seconds DeltaSeconds))
  (Default|UpdatePhisic (Variables|Default|GetEngine) _output_get (Variables|input|GetThrottle) 0.0)
  (CallFunction|CameraFunction)
  (CallFunction|UpdateWheelMesh)
  (Default|UpdatePhysic (Variables|Default|GetClutch) 0.0 (Variables|/Game/Game/Blueprints/Cars/TestCar/Engine.Engine_C|GetEngineAngularVelocityStartDWS (Variables|Default|GetEngine)) (Variables|/Game/Game/Blueprints/Cars/TestCar/GearBox.GearBox_C|GetRatio (Variables|Default|GetGearBox)))
  (Development|PrintString (Utilities|String|Append "Boost: " (Utilities|String|ToString(Float) (Variables|Default|GetBoost))) true true "(R=0.000000,G=0.000000,B=0.000000,A=1.000000)" 0.0)
  (bind _outputtorque (Default|GetOutputTorque (Variables|Default|GetGearBox) (Variables|/Game/Game/Blueprints/Cars/TestCar/Clutch.Clutch_C|GetClutchTorque (Variables|Default|GetClutch))))
  (bind (_outputtorqueleft _outputtorqueright) (Default|GetOutputTorque (Variables|Default|GetDifferential) _outputtorque))
  (Default|UpdatePhysic (Variables|Default|GetWheel_FL) (Variables|Default|GetDelta%20Seconds) 0.0 _output)
  (Default|UpdatePhysic (Variables|Default|GetWheel_FR) (Variables|Default|GetDelta%20Seconds) 0.0 _output)
  (Default|UpdatePhysic (Variables|Default|GetWheel_RL) (Variables|Default|GetDelta%20Seconds) (* _outputtorqueright _boost) _output_2)
  (Default|UpdatePhysic (Variables|Default|GetWheel_RR) (Variables|Default|GetDelta%20Seconds) (* _outputtorqueleft _boost) _output_2)
  (bind _inputshaftvelocity (Default|GetInputShaftVelocity (Variables|Default|GetDifferential) (Variables|/Game/Game/Blueprints/Cars/TestCar/Wheel.Wheel_C|GetWheelAngularVelocity (Variables|Default|GetWheel_RL)) (Variables|/Game/Game/Blueprints/Cars/TestCar/Wheel.Wheel_C|GetWheelAngularVelocity (Variables|Default|GetWheel_RR))))
  (bind _inputshaftvelocity_2 (Default|GetInputShaftVelocity _gearbox _inputshaftvelocity))
  (Default|UpdatePhysic (Variables|Default|GetClutch) _inputshaftvelocity_2 (Variables|/Game/Game/Blueprints/Cars/TestCar/Engine.Engine_C|GetEngineAngularVelocityStartDWS (Variables|Default|GetEngine)) (Variables|/Game/Game/Blueprints/Cars/TestCar/GearBox.GearBox_C|GetRatio _gearbox))
  (Default|UpdatePhisic (Variables|Default|GetEngine) (Variables|Default|GetDelta%20Seconds) (Variables|input|GetThrottle) (Variables|/Game/Game/Blueprints/Cars/TestCar/Clutch.Clutch_C|GetClutchTorque (Variables|Default|GetClutch)))
  (Development|PrintString (Utilities|String|Append "RPM: " (Utilities|String|ToString(Float) (Variables|/Game/Game/Blueprints/Cars/TestCar/Engine.Engine_C|GetEngineRPM _engine))) true true "(R=0.000000,G=0.660000,B=1.000000,A=1.000000)" 0.0)
  (Development|PrintString (Utilities|String|Append "Torque: " (Utilities|String|ToString(Float) (Variables|/Game/Game/Blueprints/Cars/TestCar/Engine.Engine_C|GetEngineEffectiveTorque _engine))) true true "(R=0.000000,G=0.660000,B=1.000000,A=1.000000)" 0.0)
  (Development|PrintString (Utilities|String|Append "GearRatio: " (Utilities|String|ToString(Float) (Variables|/Game/Game/Blueprints/Cars/TestCar/GearBox.GearBox_C|GetRatio (Variables|Default|GetGearBox)))) true true "(R=1.000000,G=0.000000,B=0.013739,A=1.000000)" 0.0)
  (Development|PrintString (Utilities|String|Append "Gear: " (Utilities|String|ToString(Text) (Variables|/Game/Game/Blueprints/Cars/TestCar/GearBox.GearBox_C|GetGearText (Variables|Default|GetGearBox)))) true true "(R=1.000000,G=0.000000,B=0.013739,A=1.000000)" 0.0)
  (Development|PrintString (Utilities|String|Append "Clutch Lock: " (Utilities|String|ToString(Float) (Variables|/Game/Game/Blueprints/Cars/TestCar/Clutch.Clutch_C|GetClutchLock _clutch))) true true "(R=0.256071,G=0.000000,B=1.000000,A=1.000000)" 0.0)
  (Development|PrintString (Utilities|String|Append "Clutch Torque: " (Utilities|String|ToString(Float) (Variables|/Game/Game/Blueprints/Cars/TestCar/Clutch.Clutch_C|GetClutchTorque _clutch))) true true "(R=0.256071,G=0.000000,B=1.000000,A=1.000000)" 0.0)
  (bind _returnvalue (Physics|GetPhysicsLinearVelocity _body "None"))
  (Development|PrintString (Utilities|String|BuildString(Integer) "Speed: " "" (Math|Float|Round (* (Math|Vector|DotProduct _returnvalue (Math|Vector|GetForwardVector _body)) 0.036)) " Km/h") true true "(R=0.958333,G=0.000000,B=0.013262,A=1.000000)" 0.0))

(event Input|AxisEvents|InputAxisSteering
  (params (AxisValue :type Float%20%28single-precision%29))
  (CallFunction|SteeringInterp AxisValue))

(event Input|AxisEvents|InputAxisBreak
  (params (AxisValue :type Float%20%28single-precision%29))
  (bind _breaktorque (Variables|Break|GetBreakTorque))
  (bind _maxbreaktorque (Variables|Break|GetMaxBreakTorque))
  (bind _breakbios (Variables|Break|GetBreakBios))
  (bind _maxbreaktorque_2 (Variables|Break|GetMaxBreakTorque))
  (bind _output_get (Variables|Break|SetBreak (Math|Interpolation|FInterptoConstant (Variables|Break|GetBreak) AxisValue (Variables|Default|GetDelta%20Seconds) (select (== AxisValue 0.0) 8.0 4.0))))
  (Development|PrintString (Utilities|String|ToString(Float) _output_get) true true "(R=0.140335,G=0.000000,B=1.000000,A=1.000000)" 0.0)
  (Utilities|Array|SetArrayElem _breaktorque 0 (* _maxbreaktorque (Variables|Break|GetBreak) _breakbios))
  (Utilities|Array|SetArrayElem _breaktorque 1 (Math|Float|Min(Float) (+ (* _maxbreaktorque (Variables|Break|GetBreak) (- 1.0 _breakbios)) (* (Input|AxisValues|GetHandBrake) _maxbreaktorque_2)) _maxbreaktorque_2)))

(event Input|AxisEvents|InputAxisThrottle
  (params (AxisValue :type Float%20%28single-precision%29))
  (bind _output_get (Variables|input|SetThrottle (Math|Interpolation|FInterptoConstant (Variables|input|GetThrottle) AxisValue (Variables|Default|GetDelta%20Seconds) (select (== AxisValue 0.0) 8.0 4.0))))
  (Development|PrintString (Utilities|String|Append "Throttle:  " (Utilities|String|ToString(Float) _output_get)) true true "(R=1.000000,G=0.000000,B=0.758377,A=1.000000)" 0.0))

(event Input|KeyboardEvents|1
  (params (Key :type Key%20Structure :default "None"))
  (:Pressed
    (Components|Activation|SetActive (Variables|Default|GetCamera1) true false)
    (Components|Activation|SetActive (Variables|Default|GetCamera) false false)
    (Components|Activation|SetActive (Variables|Default|GetCamera2) false false)))

(event Input|KeyboardEvents|2
  (params (Key :type Key%20Structure :default "None"))
  (:Pressed
    (Components|Activation|SetActive (Variables|Default|GetCamera1) false false)
    (Components|Activation|SetActive (Variables|Default|GetCamera) false false)
    (Components|Activation|SetActive (Variables|Default|GetCamera2) true false)))

(event Input|KeyboardEvents|3
  (params (Key :type Key%20Structure :default "None"))
  (:Pressed
    (Components|Activation|SetActive (Variables|Default|GetCamera1) false false)
    (Components|Activation|SetActive (Variables|Default|GetCamera) true false)
    (Components|Activation|SetActive (Variables|Default|GetCamera2) false false)))

(event Input|KeyboardEvents|E
  (params (Key :type Key%20Structure :default "None"))
  (:Pressed
    (Default|ShiftGearUp (Variables|Default|GetGearBox))))

(event Input|KeyboardEvents|Q
  (params (Key :type Key%20Structure :default "None"))
  (:Pressed
    (Default|ShiftGearDown (Variables|Default|GetGearBox))))

(event Input|KeyboardEvents|LeftShift
  (params (Key :type Key%20Structure :default "None"))
  (:Pressed
    (Variables|Default|SetBoost 5.0))
  (:Released
    (Variables|Default|SetBoost 1.0)))

(event Input|KeyboardEvents|C
  (params (Key :type Key%20Structure :default "None")))

(fn ConstructionScript
  (for _index (range 0 3)
    (bind _returnvalue (AddComponent|AddStaticMeshComponent false))
    (Components|StaticMesh|SetStaticMesh _returnvalue (Variables|Wheel|GetWheelMesh))
    (Collision|SetCollisionEnabled _returnvalue "NoCollision")
    (Transformation|SetRelativeScale3D _returnvalue (Math|Vector|MakeVector 1.0 (Utilities|Select :Index _index :Option%200 -1.0 :Option%201 1.0 :Option%202 -1.0 :Option%203 1.0) 1.0))
    (Transformation|SetRelativeLocation _returnvalue (Math|Vector|MakeVector 0.0 0.0 (* (Variables|/Game/Game/Blueprints/Cars/TestCar/Wheel.Wheel_C|GetRestLenght (Utilities|Select :Index _index :Option%200 (Variables|Default|GetWheel_FL) :Option%201 (Variables|Default|GetWheel_FR) :Option%202 (Variables|Default|GetWheel_RL) :Option%203 (Variables|Default|GetWheel_RR))) -1.0)) false false)
    (Transformation|AttachComponentToComponent _returnvalue (Utilities|Select :Index _index :Option%200 (Variables|Default|GetWheel_FL) :Option%201 (Variables|Default|GetWheel_FR) :Option%202 (Variables|Default|GetWheel_RL) :Option%203 (Variables|Default|GetWheel_RR)) "None" "KeepRelative" "KeepRelative" "KeepRelative" true)))

(fn CameraFunction
  (bind _springarm (Variables|Default|GetSpringArm))
  (bind _relativerotation (Variables|/Script/Engine.SceneComponent|GetRelativeRotation _springarm))
  (Transformation|SetRelativeRotation _springarm (Math|Rotator|MakeRotator (.roll _relativerotation) (Math|Float|Clamp(Float) (+ (Class|Actor|GetInputAxisKeyValue) (.pitch _relativerotation)) -6e+01 6e+01) (+ (.yaw _relativerotation) (Class|Actor|GetInputAxisKeyValue))) false false))

(fn UpdateWheelMesh
  (for _index (range 0 3)
    (Transformation|SetRelativeLocation (Components|GetChildComponent (Utilities|Select :Index _index :Option%200 (Variables|Default|GetWheel_FL) :Option%201 (Variables|Default|GetWheel_FR) :Option%202 (Variables|Default|GetWheel_RL) :Option%203 (Variables|Default|GetWheel_RR)) 0) (Math|Vector|MakeVector 0.0 0.0 (* (Variables|/Game/Game/Blueprints/Cars/TestCar/Wheel.Wheel_C|GetCurrentLength (Utilities|Select :Index _index :Option%200 (Variables|Default|GetWheel_FL) :Option%201 (Variables|Default|GetWheel_FR) :Option%202 (Variables|Default|GetWheel_RL) :Option%203 (Variables|Default|GetWheel_RR))) -1.0)) false false)
    (Transformation|AddLocalRotation (Components|GetChildComponent (Utilities|Select :Index _index :Option%200 (Variables|Default|GetWheel_FL) :Option%201 (Variables|Default|GetWheel_FR) :Option%202 (Variables|Default|GetWheel_RL) :Option%203 (Variables|Default|GetWheel_RR)) 0) (Math|Rotator|MakeRotator 0.0 (* (Math|Trig|RadiansToDegrees (Variables|/Game/Game/Blueprints/Cars/TestCar/Wheel.Wheel_C|GetWheelAngularVelocity (Utilities|Select :Index _index :Option%200 (Variables|Default|GetWheel_FL) :Option%201 (Variables|Default|GetWheel_FR) :Option%202 (Variables|Default|GetWheel_RL) :Option%203 (Variables|Default|GetWheel_RR)))) (Variables|Default|GetDelta%20Seconds) -1.0) 0.0) false false)))

(fn SteeringInterp
  (params (Axis :type Float%20%28single-precision%29))
  (bind _delta_seconds (Variables|Default|GetDelta%20Seconds))
  (bind _output_get (Variables|input|SetSteeringAngle (Math|Interpolation|FInterpTo (Variables|input|GetSteeringAngle) (* Axis (Variables|Default|GetMaxSteeringAngle)) _delta_seconds (* (/ 1.0 _delta_seconds) (select (== Axis 0.0) 0.3 0.04)))))
  (Transformation|SetRelativeRotation (Variables|Default|GetWheel_FR) (Math|Rotator|MakeRotator 0.0 0.0 _output_get) false false))